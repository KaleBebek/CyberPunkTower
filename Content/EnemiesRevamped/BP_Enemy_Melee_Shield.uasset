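; Sword-and-shield melee enemy, a child Blueprint that sets its own health, EXP value, combat ranges and movement speeds.
; On BeginPlay it spawns both weapons onto hand sockets, with WeaponActor ending up as the shield.
; Attacks play an uninterruptible montage whose Slash notify sphere-traces forward to deal damage, with debug drawing on.
; Blocking toggles the damage component's flag and turns the shield gold; blocked hits spawn a particle effect.
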(event OnBlocked(BPC_DamageSystem)
  (params (CanBeParried :type Boolean) (DamageCauser :type Actor%20Object%20Reference))
  (Effects|SpawnEmitteratLocation "/Game/P_SparrowPrimaryMuzzleFlash.P_SparrowPrimaryMuzzleFlash" (Transformation|GetActorLocation)))

(event Custom|End%20Block
  (Variables|/Game/DamageSystem/BPC_DamageSystem.BPC_DamageSystem_C|SetIsBlocking (Variables|Default|GetBPC_DamageSystem) false)
  (Rendering|Material|SetMaterial (Variables|/Game/Weapons/BP_Weapon_Base.BP_Weapon_Base_C|GetMesh (stale EventEquipWeapon _returnvalue_2)) 0 "/Game/StarterContent/Materials/M_Metal_Steel.M_Metal_Steel"))

(event Custom|StartBlocking
  (Rendering|Material|SetMaterial (Variables|/Game/Weapons/BP_Weapon_Base.BP_Weapon_Base_C|GetMesh (stale EventEquipWeapon _returnvalue_2)) 0 "/Game/StarterContent/Materials/M_Metal_Gold.M_Metal_Gold")
  (Variables|/Game/DamageSystem/BPC_DamageSystem.BPC_DamageSystem_C|SetIsBlocking (Variables|Default|GetBPC_DamageSystem) true))

(event EventEquipWeapon
  (Utilities|FlowControl|Sequence
    (:then_0
      (bind _returnvalue (Game|SpawnActorfromClass "/Game/Weapons/BP_Weapon_Sword.BP_Weapon_Sword_C" (Transformation|GetActorTransform) "Undefined" "MultiplyWithRoot" 0 0))
      (bind _output_get (Variables|Default|SetWeaponActor _returnvalue))
      (Transformation|AttachComponentToComponent _output_get (Variables|Character|GetMesh) "hand_r_sword_socket" "SnapToTarget" "SnapToTarget" "SnapToTarget" true)
      (Variables|Default|SetIsWeaponEquipped? true)
      (Default|CallOnWeaponEquipped))
    (:then_1
      (bind _returnvalue_2 (Game|SpawnActorfromClass "/Game/Weapons/BP_Weapon_Shield.BP_Weapon_Shield_C" (Transformation|GetActorTransform) "Undefined" "MultiplyWithRoot" 0 0))
      (bind _output_get_2 (Variables|Default|SetWeaponActor _returnvalue_2))
      (Transformation|AttachComponentToComponent _output_get_2 (Variables|Character|GetMesh) "hand_l_shield_socket" "SnapToTarget" "SnapToTarget" "SnapToTarget" true))))

(event EventBeginPlay
  (|CallParentFunction)
  (Variables|Default|SetExpValue 100)
  (CallFunction|EquipWeapon))

(event EventAttack
  (params (AttackTarget :type Actor%20Object%20Reference))
  (bind _returnvalue (Transformation|GetActorLocation))
  (Variables|Default|SetAttacking true)
  (bind _notifyname (Animation|Montage|PlayMontage (Variables|Character|GetMesh) "/Game/EnemiesRevamped/Animations/Sword_Shield_Slash_Montage.Sword_Shield_Slash_Montage")
    (:then
      (Variables|/Game/DamageSystem/BPC_DamageSystem.BPC_DamageSystem_C|SetIsInterruptible (Variables|Default|GetBPC_DamageSystem) false))
    (:OnCompleted
      (Default|CallOnAttackEnd :!label _label)
      (Variables|/Game/DamageSystem/BPC_DamageSystem.BPC_DamageSystem_C|SetIsInterruptible (Variables|Default|GetBPC_DamageSystem) true)
      (Variables|Default|SetAttacking false))
    (:OnInterrupted
      (goto _label))
    (:OnNotifyBegin
      (switch name _notifyname
        (:Slash
          (bind (_outhit _returnvalue_2) (Collision|SphereTraceForObjects _returnvalue (+ _returnvalue (* (Transformation|GetActorForwardVector) 2e+02)) 2e+01 (Utilities|Array|MakeArray "ObjectTypeQuery3") false 0 "ForDuration"))
          (if _returnvalue_2
            (Class|BPIDamagable|TakeDamage(Message) (.HitActor (Collision|BreakHitResult _outhit)) (Utilities|Struct|MakeS_DamageInfo 25.0 "NewEnumerator1") self)))))))

(fn ConstructionScript
  (bind _bpc_damagesystem (Variables|Default|GetBPC_DamageSystem))
  (|CallParentFunction)
  (bind _output_get (Variables|/Game/DamageSystem/BPC_DamageSystem.BPC_DamageSystem_C|SetMaxHealth _bpc_damagesystem 1e+02))
  (Variables|/Game/DamageSystem/BPC_DamageSystem.BPC_DamageSystem_C|SetHealth _bpc_damagesystem _output_get))

(fn GetIdealRange
  (return 1e+02 4e+02))

(fn SetMovementSpeed
  (params (Speed :type E_MovementSpeed%20Enum :default "NewEnumerator0"))
  (bind _output_get (Variables|/Script/Engine.CharacterMovementComponent|SetMaxWalkSpeed (Variables|Character|GetCharacterMovement) (Utilities|Select :Index Speed :NewEnumerator0 0.0 :NewEnumerator1 1e+02 :NewEnumerator2 3e+02 :NewEnumerator3 4e+02 :NewEnumerator4 2e+02)))
  (return _output_get))