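; Mage enemy Blueprint that sets its own stats and ideal ranges, with fireball, barrage and ground smash attacks run through BPCAttacks.
; Teleport is faked by fast AI-driven flight with the mesh hidden, invincibility, no pawn collision and a steam effect, all reverted on move success or failure.
; Healing plays a montage and spawns a floor AOE whose overlap ticks heal only the mage by a percentage of max health.
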(event Custom|Teleport
  (params (Destination :type Vector))
  (bind _bpc_damagesystem (Variables|Default|GetBPC_DamageSystem))
  (bind _charactermovement (Variables|Character|GetCharacterMovement))
  (bind _mesh (Variables|Character|GetMesh))
  (Variables|/Game/DamageSystem/BPC_DamageSystem.BPC_DamageSystem_C|SetIsInterruptible _bpc_damagesystem false)
  (Variables|/Game/DamageSystem/BPC_DamageSystem.BPC_DamageSystem_C|SetIsInvincible _bpc_damagesystem true)
  (if (not (Variables|Default|GetIsTeleporting?))
    (Variables|Default|SetIsTeleporting? true)
    (Pawn|Components|CharacterMovement|SetMovementMode _charactermovement "MOVE_Flying" 0)
    (Variables|/Script/Engine.CharacterMovementComponent|SetMaxFlySpeed _charactermovement 4e+03)
    (Variables|/Script/Engine.CharacterMovementComponent|SetMaxAcceleration _charactermovement 99999.0)
    (Rendering|SetVisibility _mesh false true)
    (Collision|SetCollisionResponsetoChannel (Variables|Default|GetCapsuleComponent) "ECC_Pawn" "ECR_Ignore")
    (bind _returnvalue (Effects|SpawnEmitterAttached "/Game/StarterContent/Particles/P_Steam_Lit.P_Steam_Lit" _mesh "Spine1"))
    (Variables|Default|SetTeleportBodyEffect _returnvalue)
    (Animation|StopAnimMontage 0)
    (AI|AIMoveTo self Destination 0 5.0 false
      (:OnSuccess
        _)
      (:OnFail
        _))
    (CallFunction|TeleportEnd)
    (else
      (Utilities|FlowControl|DelayUntilNextTick)
      (Default|CallOnTeleportEnd))))

(event Custom|TeleportEnd
  (bind _bpc_damagesystem (Variables|Default|GetBPC_DamageSystem))
  (bind _charactermovement (Variables|Character|GetCharacterMovement))
  (Variables|/Game/DamageSystem/BPC_DamageSystem.BPC_DamageSystem_C|SetIsInterruptible _bpc_damagesystem true)
  (Variables|/Game/DamageSystem/BPC_DamageSystem.BPC_DamageSystem_C|SetIsInvincible _bpc_damagesystem false)
  (Components|Movement|StopMovementImmediately _charactermovement)
  (Pawn|Components|CharacterMovement|SetMovementMode _charactermovement "MOVE_Walking" 0)
  (Variables|/Script/Engine.CharacterMovementComponent|SetMaxAcceleration _charactermovement 1.5e+03)
  (Rendering|SetVisibility (Variables|Character|GetMesh) true true)
  (Collision|SetCollisionResponsetoChannel (Variables|Default|GetCapsuleComponent) "ECC_Pawn" "ECR_Block")
  (Default|CallOnTeleportEnd)
  (Variables|Default|SetIsTeleporting? false)
  (bind _teleportbodyeffect (Variables|Default|GetTeleportBodyEffect)
    (:then
      (Components|DestroyComponent _teleportbodyeffect))
    (:else)))

(event Custom|HealOverTime
  (params (HealPercentage :type Float%20%28double-precision%29))
  (bind _returnvalue (Transformation|GetActorLocation))
  (Animation|Montage|PlayMontage (Variables|Character|GetMesh) "/Game/Characters/Mage/Animations/Montages/Montage_Mage_Heal.Montage_Mage_Heal"
    (:then
      (bind (_outhit _returnvalue_2) (Collision|LineTraceByChannel _returnvalue (* _returnvalue "0.000000,0.000000,-1000.000000") "TraceTypeQuery1" false 0 "ForDuration"))
      (if _returnvalue_2
        (bind _returnvalue_3 (Game|SpawnActorfromClass "/Game/EnemiesRevamped/AOE/BP_AOE_Heal.BP_AOE_Heal_C" (Math|Transform|MakeTransform (.Location (Collision|BreakHitResult _outhit)) "0, 0, 0" "1.000000,1.000000,1.000000") "Undefined" "MultiplyWithRoot" 0 0.2 1e+01 false false true 0))
        (bind _output_get (Variables|Default|SetHealAOE _returnvalue_3))
        (EventDispatchers|AssignOnAOEOverlapActor _output_get (delegate Custom|OnHealTick))
        (else
          (Animation|StopAnimMontage 0))))
    (:OnCompleted
      (CallFunction|HealOverTimeEnd :!label _label))
    (:OnInterrupted
      (goto _label))))

(event Custom|HealOverTimeEnd
  (Default|CallOnHealOvertimeEnds)
  (bind _healaoe (Variables|Default|GetHealAOE)
    (:then
      (Actor|DestroyActor _healaoe))
    (:else)))

(event Custom|OnHealTick
  (params (Actor :type Actor%20Object%20Reference))
  (if (== Actor self)
    (CallFunction|Heal (* (Variables|/Game/DamageSystem/BPC_DamageSystem.BPC_DamageSystem_C|GetMaxHealth (Variables|Default|GetBPC_DamageSystem)) (stale Custom|HealOverTime HealPercentage)))))

(event Custom|BasicAttack
  (params (AttackTarget :type Actor%20Object%20Reference))
  ;[1 1 1] Attacks
  (Default|BasicMageAttack (Variables|Default|GetBPC_Attacks) (Utilities|Struct|MakeS_AttackInfo AttackTarget "/Game/Characters/Mage/Animations/Montages/Montage_Mage_Fireball.Montage_Mage_Fireball" (Utilities|Struct|MakeS_DamageInfo (Variables|Default|GetBaseAttackDamage) "NewEnumerator2")) 2e+03))

(event Custom|BarrageAttack
  (params (AttackTarget :type Actor%20Object%20Reference))
  ;[1 1 1] Attacks
  (Default|MageBarrageAttack (Variables|Default|GetBPC_Attacks) (Utilities|Struct|MakeS_AttackInfo AttackTarget "/Game/Characters/Mage/Animations/Montages/Montage_Mage_Barrage_Attack.Montage_Mage_Barrage_Attack" (Utilities|Struct|MakeS_DamageInfo (* (Variables|Default|GetBaseAttackDamage) 2.0) "NewEnumerator2")) 2.5e+03))

(event Custom|GroundSmashAttack
  (params (Attack%20Target :type Actor%20Object%20Reference))
  ;[1 1 1] Attacks
  (Default|GroundSmash (Variables|Default|GetBPC_Attacks) (Utilities|Struct|MakeS_AttackInfo Attack%20Target "/Game/Characters/Mage/Animations/Montage_Mage_GroundSmash.Montage_Mage_GroundSmash" (Utilities|Struct|MakeS_DamageInfo (* (Variables|Default|GetBaseAttackDamage) 3.0) "NewEnumerator3")) 3e+02))

(event EventBeginPlay
  (|CallParentFunction)
  (Variables|Default|SetIsWeaponEquipped? true) ; Weapon is hands for now
  (CallFunction|CalculateEnemyStats 5e+01 3.0 100 50))

(fn ConstructionScript)

(fn SetMovementSpeed
  (params (Speed :type E_MovementSpeed%20Enum :default "NewEnumerator0"))
  (bind _output_get (Variables|/Script/Engine.CharacterMovementComponent|SetMaxWalkSpeed (Variables|Character|GetCharacterMovement) (Utilities|Select :Index Speed :NewEnumerator0 0.0 :NewEnumerator1 1e+02 :NewEnumerator2 3e+02 :NewEnumerator3 5e+02 :NewEnumerator4 3e+02)))
  (return _output_get))

(fn GetIdealRange
  (return 1e+03 6e+02))