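; Ranged flying enemy Blueprint that spawns a rifle on BeginPlay, attaches it to its hand socket and sets its experience value.
; Its Attack override plays a fire montage whose Fire notify line-traces from weapon to target, damaging the target only when the trace hits nothing, then calls AttackEnd on completion or interruption.
; It also supplies attack and strafe ranges and maps movement states to MaxWalkSpeed, despite the flying name.
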(event EventBeginPlay
  (|CallParentFunction)
  (CallFunction|EquipWeapon)
  (Variables|Default|SetExpValue 25))

(event EventEquipWeapon
  (bind _returnvalue (Game|SpawnActorfromClass "/Game/Weapons/BP_Weapon_Rifle.BP_Weapon_Rifle_C" (Math|Transform|MakeTransform "0, 0, 0") "Undefined" "MultiplyWithRoot" 0 0))
  (bind _output_get (Variables|Default|SetWeaponActor _returnvalue))
  (Transformation|AttachComponentToComponent _output_get (Variables|Character|GetMesh) "hand_r_rifle_socket" "SnapToTarget" "SnapToTarget" "SnapToTarget" true)
  (Variables|Default|SetIsWeaponEquipped? true)
  (Default|CallOnWeaponEquipped))

(event EventAttack
  (params (AttackTarget :type Actor%20Object%20Reference))
  (|CallParentFunction AttackTarget)
  (bind _notifyname (Animation|Montage|PlayMontage (Variables|Character|GetMesh) "/Game/EnemiesRevamped/Animations/Rifle-Fire_Montage.Rifle-Fire_Montage")
    (:OnCompleted
      (CallFunction|AttackEnd AttackTarget :!label _label))
    (:OnInterrupted
      (goto _label))
    (:OnNotifyBegin
      (switch name _notifyname
        (:Fire
          (bind _returnvalue (Collision|LineTraceByChannel (Transformation|GetActorLocation (Variables|Default|GetWeaponActor)) (Transformation|GetActorLocation AttackTarget) "TraceTypeQuery1" false 0 "ForDuration" true "(R=1.000000,G=0.000000,B=0.000000,A=1.000000)" "(R=0.000000,G=1.000000,B=0.000000,A=1.000000)" 3.0))
          (if (not _returnvalue)
            (Class|BPIDamagable|TakeDamage(Message) AttackTarget (Utilities|Struct|MakeS_DamageInfo 1e+01 "NewEnumerator2") self)))))))

(fn ConstructionScript
  (|CallParentFunction))

(fn SetMovementSpeed
  (params (Speed :type E_MovementSpeed%20Enum :default "NewEnumerator0"))
  (bind _output_get (Variables|/Script/Engine.CharacterMovementComponent|SetMaxWalkSpeed (Variables|Character|GetCharacterMovement) (Utilities|Select :Index Speed :NewEnumerator0 0.0 :NewEnumerator1 1e+01 :NewEnumerator2 1e+01 :NewEnumerator3 1e+01 :NewEnumerator4 1e+01)))
  (return _output_get))

(fn GetIdealRange
  (return 1e+03 5e+02))