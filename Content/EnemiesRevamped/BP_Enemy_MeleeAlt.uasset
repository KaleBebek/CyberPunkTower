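; BP_Enemy_MeleeAlt is a sword-wielding melee enemy that sets its stats through CalculateEnemyStats on BeginPlay.
; Its basic, spinning and ground smash attack events pass montage and damage info to BPCAttacks.
; Equip and unequip montages use notifies to spawn and socket or destroy the sword, then signal on completion.
; It also supplies ideal attack and strafe ranges and maps speed states to walk speeds.
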(event Custom|SpinningAttack
  (params (AttackTarget :type Actor%20Object%20Reference))
  (Default|SpinningAttack (Variables|Default|GetBPC_Attacks) (Utilities|Struct|MakeS_AttackInfo AttackTarget "/Game/EnemiesRevamped/Animations/Montage_Sword_SpinningAttack.Montage_Sword_SpinningAttack" (Utilities|Struct|MakeS_DamageInfo 1e+01 "NewEnumerator1")) 3e+02))

(event Custom|GroundSmashAttack
  (params (AttackTarget :type Actor%20Object%20Reference))
  (Default|GroundSmash (Variables|Default|GetBPC_Attacks) (Utilities|Struct|MakeS_AttackInfo AttackTarget "/Game/EnemiesRevamped/Animations/Sword_Ground_Smash_Montage.Sword_Ground_Smash_Montage" (Utilities|Struct|MakeS_DamageInfo 1e+01 "NewEnumerator1")) 3e+02))

(event Custom|BasicAttack
  (params (AttackTarget :type Actor%20Object%20Reference))
  (Default|BasicMeleeAttack (Variables|Default|GetBPC_Attacks) (Utilities|Struct|MakeS_AttackInfo AttackTarget "/Game/EnemiesRevamped/Animations/Sword_Slash_Montage.Sword_Slash_Montage" (Utilities|Struct|MakeS_DamageInfo 1e+01 "NewEnumerator1")) 2e+01 2e+02))

(event EventUnequipWeapon
  (bind _notifyname (Animation|Montage|PlayMontage (Variables|Character|GetMesh) "/Game/EnemiesRevamped/Animations/Sheath_Sword_Montage.Sheath_Sword_Montage")
    (:OnCompleted
      (Default|CallOnWeaponUnequipped))
    (:OnNotifyBegin
      (switch name _notifyname
        (:RemoveSword
          (Actor|DestroyActor (Variables|Default|GetWeaponActor))
          (Variables|Default|SetIsWeaponEquipped? false))))))

(event EventBeginPlay
  (|CallParentFunction)
  (CallFunction|CalculateEnemyStats 5e+01 1.0 50 20))

(event EventEquipWeapon
  (bind _notifyname (Animation|Montage|PlayMontage (Variables|Character|GetMesh) "/Game/EnemiesRevamped/Animations/Unsheath_Sword_Montage.Unsheath_Sword_Montage")
    (:OnCompleted
      (Default|CallOnWeaponEquipped))
    (:OnNotifyBegin
      (switch name _notifyname
        (:HoldSword
          (bind _returnvalue (Game|SpawnActorfromClass "/Game/Weapons/BP_Weapon_Sword.BP_Weapon_Sword_C" (Transformation|GetActorTransform) "Undefined" "MultiplyWithRoot" 0 0))
          (bind _output_get (Variables|Default|SetWeaponActor _returnvalue))
          (Transformation|AttachComponentToComponent _output_get (Variables|Character|GetMesh) "hand_r_sword_socket" "SnapToTarget" "SnapToTarget" "SnapToTarget" true)
          (Variables|Default|SetIsWeaponEquipped? true))))))

(fn ConstructionScript)

(fn GetIdealRange
  (return 1.5e+02 3.5e+02))

(fn SetMovementSpeed
  (params (Speed :type E_MovementSpeed%20Enum :default "NewEnumerator0"))
  (bind _output_get (Variables|/Script/Engine.CharacterMovementComponent|SetMaxWalkSpeed (Variables|Character|GetCharacterMovement) (Utilities|Select :Index Speed :NewEnumerator0 0.0 :NewEnumerator1 1e+02 :NewEnumerator2 3e+02 :NewEnumerator3 5e+02 :NewEnumerator4 2e+02)))
  (return _output_get))