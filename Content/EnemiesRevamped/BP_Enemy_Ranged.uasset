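; BP_Enemy_Ranged is a rifle-wielding enemy that extends a parent enemy Blueprint with ranged combat, its own health, rewards, movement speeds and ideal combat range.
; On BeginPlay it spawns a rifle, attaches it to a hand socket and signals that the weapon is equipped.
; Attack plays a fire montage whose notify fires a projectile from the weapon at the target through BPCAttacks, and ends the attack on completion or interruption.
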(event EventBeginPlay
  (|CallParentFunction)
  (CallFunction|EquipWeapon)
  (Variables|Default|SetExpValue 25)
  (Variables|Default|SetCreditsValue 7))

(event EventEquipWeapon
  (bind _returnvalue (Game|SpawnActorfromClass "/Game/Weapons/BP_Weapon_Rifle.BP_Weapon_Rifle_C" (Math|Transform|MakeTransform "0, 0, 0") "Undefined" "MultiplyWithRoot" 0 0))
  (bind _output_get (Variables|Default|SetWeaponActor _returnvalue))
  (Transformation|AttachComponentToComponent _output_get (Variables|Character|GetMesh) "hand_r_rifle_socket" "SnapToTarget" "SnapToTarget" "SnapToTarget" true)
  (Variables|Default|SetIsWeaponEquipped? true)
  (Default|CallOnWeaponEquipped))

(event EventAttack
  (params (AttackTarget :type Actor%20Object%20Reference))
  (|CallParentFunction AttackTarget)
  (bind _notifyname (Animation|Montage|PlayMontage (Variables|Character|GetMesh) "/Game/EnemiesRevamped/Animations/Rifle-Fire_Montage.Rifle-Fire_Montage")
    (:OnCompleted
      (CallFunction|AttackEnd AttackTarget :!label _label))
    (:OnInterrupted
      (goto _label))
    (:OnNotifyBegin
      (switch name _notifyname
        (:Fire
          (Default|BasicProjectile (Variables|Default|GetBPC_Attacks) (Utilities|Struct|MakeS_DamageInfo 15.0 "NewEnumerator2") (Math|Transform|MakeTransform (Transformation|GetActorLocation (Variables|Default|GetWeaponActor)) "0, 0, 0" "1.000000,1.000000,1.000000") AttackTarget))))))

(fn ConstructionScript
  (bind _bpc_damagesystem (Variables|Default|GetBPC_DamageSystem))
  (|CallParentFunction)
  (bind _output_get (Variables|/Game/DamageSystem/BPC_DamageSystem.BPC_DamageSystem_C|SetMaxHealth _bpc_damagesystem 8e+01))
  (Variables|/Game/DamageSystem/BPC_DamageSystem.BPC_DamageSystem_C|SetHealth _bpc_damagesystem _output_get))

(fn SetMovementSpeed
  (params (Speed :type E_MovementSpeed%20Enum :default "NewEnumerator0"))
  (bind _output_get (Variables|/Script/Engine.CharacterMovementComponent|SetMaxWalkSpeed (Variables|Character|GetCharacterMovement) (Utilities|Select :Index Speed :NewEnumerator0 0.0 :NewEnumerator1 1e+02 :NewEnumerator2 3e+02 :NewEnumerator3 5e+02 :NewEnumerator4 3e+02)))
  (return _output_get))

(fn GetIdealRange
  (return 8e+02 8e+02))