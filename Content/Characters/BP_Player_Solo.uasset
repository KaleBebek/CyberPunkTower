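; Solo player character Blueprint, extending a parent with one-time stat modifiers, a HUD and music outside the main menu.
; Primary, rocket, homing barrage, shockwave and directional dodge-roll inputs use DoOnce-plus-Delay cooldowns, sending attacks with calculated damage to BPCAttacks and most cooldowns to the HUD.
; Damage responses start timer-based health regen.
; Death ragdolls the player, records the killer, zooms out, freezes time and shows game over.
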(event OnDeath(BPC_DamageSystem)
  (bind _returnvalue (Game|GetPlayerController 0))
  ;[1 0.1456 0.1655] Death stuff
  (Utilities|Time|ClearandInvalidateTimerbyHandle (Variables|/Game/Attacks/BPC_Attacks.BPC_Attacks_C|GetGunTimerReference (Variables|Default|GetBPC_Attacks)))
  (CallFunction|RagdollDeath)
  (Audio|PlaySound2D "/Game/Sounds/elevatording_Cue.elevatording_Cue" 0.2 1.0 0.0 0 0) ; dead
  (Variables|Default|SetIsDead? true)
  (Widget|RemovefromParent (Variables|Default|GetHUDRef))
  (bind _asmy_game_instance (Utilities|Casting|CastToMyGameInstance (Game|GetGameInstance)))
  (Variables|/Game/Blueprints/MyGameInstance.MyGameInstance_C|SetKilledBy _asmy_game_instance (Utilities|GetDisplayName (Variables|Default|GetDamage%20Causer)))
  (bind _zoom_out (Timeline|Timeline PlayFromStart)
    (:Update
      (Variables|/Script/Engine.SpringArmComponent|SetTargetArmLength (Variables|Default|GetCameraBoom) (Math|Float|Lerp 4e+02 7e+02 _zoom_out))
      (Utilities|FlowControl|Delay 3.0)
      (Utilities|Time|SetGlobalTimeDilation 0.0)
      (bind _returnvalue_2 (UserInterface|CreateWidget "/Game/UI_Widgets/GameOver_UI.GameOver_UI_C"))
      (UserInterface|Viewport|AddtoViewport _returnvalue_2 0)
      (Input|SetInputModeUIOnly _returnvalue 0 "DoNotLock" false)
      (Variables|/Script/Engine.PlayerController|SetbShowMouseCursor _returnvalue true)
      (Default|ResetGameDefaults _asmy_game_instance))))

(event OnDamageResponse(BPC_DamageSystem)
  (params (DamageResponse :type E_DamageResponse%20Enum :default "NewEnumerator0") (DamageCauser :type Actor%20Object%20Reference) (Amount :type Float%20%28double-precision%29) (Interuptible :type Boolean))
  ;[1 1 1] Heal over time
  (Variables|Default|SetDamage%20Causer DamageCauser)
  (CallFunction|StartHealing))

(event Custom|StartHealing
  (bind _bpc_damagesystem (Variables|Default|GetBPC_DamageSystem))
  ;[1 1 1] Heal over time
  (if (< (Variables|/Game/DamageSystem/BPC_DamageSystem.BPC_DamageSystem_C|GetHealth _bpc_damagesystem) (Variables|/Game/DamageSystem/BPC_DamageSystem.BPC_DamageSystem_C|GetMaxHealth _bpc_damagesystem))
    (bind _returnvalue (Utilities|Time|SetTimerbyFunctionName 0 "HealthRegen" 2.0 true))
    (else
      (Utilities|Time|ClearandInvalidateTimerbyHandle _returnvalue))))

(event EventBeginPlay
  ;[0.2622 1 0.2689] Player Initialization
  (|CallParentFunction)
  (if (not (Utilities|Enum|Equal(Enum) (Utilities|GetDisplayName (Game|GetGameMode)) "MenuGameMode_C_0"))
    (CallFunction|AddSoloModifiers)
    (bind _returnvalue (UserInterface|CreateWidget "/Game/UI_Widgets/BasicHUD_UI.BasicHUD_UI_C" 0 self)) ; create this characters hud
    (bind _output_get (Variables|Default|SetHUDRef _returnvalue))
    (UserInterface|Viewport|AddtoViewport _output_get 0)
    (bind _returnvalue_2 (Audio|SpawnSound2D 0 0.05 1.0 0.0 0)) ; in game music goes here
    (Variables|Default|SetBackgroundAudio _returnvalue_2)))

(event Input|ActionEvents|InputActionPrimaryShoot
  (params (Key :type Key%20Structure :default "None"))
  (bind _fire_rate (Variables|Default|GetFire%20Rate))
  ;[0.02745 0.6549 1] Primary Fire (Limits user from spam clicking before shooting again)
  (:Pressed
    (if (not (Variables|Default|GetIsDead?))
      (Utilities|FlowControl|Sequence
        (:then_0
          (Utilities|FlowControl|DoOnce false :!label _label
            (:Completed
              (bind _damage (CallFunction|CalculateDamage (Variables|Default|GetAttackDamage) (Variables|Default|GetCritChance) (Variables|Default|GetLifeSteal)))
              (Default|PlayerPrimary (Variables|Default|GetBPC_Attacks) (Utilities|Struct|MakeS_DamageInfo _damage "NewEnumerator2" "NewEnumerator0" false true) (Variables|Default|GetFollowCamera) (Variables|Default|GetWeapon%20Range) _fire_rate))))
        (:then_1
          (Utilities|FlowControl|Delay _fire_rate)
          (goto _label Reset)))))
  (:Released
    (Default|StopShooting (Variables|Default|GetBPC_Attacks))))

(event Input|ActionEvents|InputActionUltimate
  (params (Key :type Key%20Structure :default "None"))
  (bind _ultimatecd (Variables|Abilities|GetUltimateCD))
  (bind _globalcooldown (Variables|Default|GetGlobalCooldown))
  (bind _homingspawnpos (Variables|Default|GetHomingSpawnPos))
  (bind _returnvalue (Transformation|GetWorldTransform _homingspawnpos))
  (bind _returnvalue_2 (* _ultimatecd _globalcooldown))
  ;[0.02745 0.6549 1] Ultimate Ability
  (:Pressed
    (if (not (Variables|Default|GetIsDead?))
      (Utilities|FlowControl|Sequence
        (:then_0
          (Utilities|FlowControl|DoOnce false :!label _label
            (:Completed
              (Default|UltimateonCooldown (Variables|Default|GetHUDRef) _returnvalue_2)
              (Audio|PlaySoundatLocation "/Game/Sounds/Missile_Barrage_3.Missile_Barrage_3" "0, 0, 0" "0, 0, 0" 0.2 1.0 0.0 0 0 0 0)
              (Utilities|ForLoopwithDelay 0 5 0.15
                (:Loop%20Body
                  (bind _damage (CallFunction|CalculateDamage (Variables|Default|GetAttackDamage) (Variables|Default|GetCritChance) (Variables|Default|GetLifeSteal)))
                  (Default|PlayerBarrage (Variables|Default|GetBPC_Attacks) (Math|Transform|MakeTransform (.location _returnvalue) (Math|Rotator|MakeRotator (.roll (.rotation _returnvalue)) (.pitch (.rotation _returnvalue)) (+ (.yaw (.rotation _returnvalue)) (Variables|Abilities|GetMissleRotation))) "1.000000,1.000000,1.000000") 0 (Utilities|Struct|MakeS_DamageInfo (* _damage 2.5) "NewEnumerator2" "NewEnumerator1") 4e+03 2e+02 5e+02)
                  (Variables|Abilities|SetMissleRotation (+ 1e+02 (Variables|Abilities|GetMissleRotation))))
                (:Completed
                  (Variables|Abilities|SetMissleRotation 0.0))))))
        (:then_1
          (Utilities|FlowControl|Delay _returnvalue_2)
          (goto _label Reset))))))

(event Input|ActionEvents|InputActionSecondaryShoot
  (params (Key :type Key%20Structure :default "None"))
  (bind _globalcooldown (Variables|Default|GetGlobalCooldown))
  (bind _projectile_spawn_pos (Variables|Default|Getprojectile%20spawn%20pos))
  (bind _secondarycd (Variables|Abilities|GetSecondaryCD))
  (bind _returnvalue (Transformation|GetWorldTransform _projectile_spawn_pos))
  (bind _returnvalue_2 (* _secondarycd _globalcooldown))
  ;[0.02745 0.6549 1] Secondary Fire
  (:Pressed
    (if (not (Variables|Default|GetIsDead?))
      (Utilities|FlowControl|Sequence
        (:then_0
          (Utilities|FlowControl|DoOnce false :!label _label
            (:Completed
              (Default|SecondaryonCooldown (Variables|Default|GetHUDRef) _returnvalue_2)
              (Class|Actor|MakeNoise 1.0 0 (.location _returnvalue) 0.0 "None") ; shot noise
              (bind _damage (CallFunction|CalculateDamage (Variables|Default|GetAttackDamage) (Variables|Default|GetCritChance) (Variables|Default|GetLifeSteal)))
              (Default|PlayerRocket (Variables|Default|GetBPC_Attacks) (Math|Transform|MakeTransform (.location _returnvalue) (Transformation|GetWorldRotation (Variables|Default|GetFollowCamera)) "1.000000,1.000000,1.000000") 0 (Utilities|Struct|MakeS_DamageInfo (* _damage 2.0) "NewEnumerator2" "NewEnumerator1") 6e+03 3e+02))))
        (:then_1
          (Utilities|FlowControl|Delay _returnvalue_2)
          (goto _label Reset))))))

(event Input|ActionEvents|InputActionAbility
  (params (Key :type Key%20Structure :default "None"))
  (bind _abilitycd (Variables|Abilities|GetAbilityCD))
  (bind _globalcooldown (Variables|Default|GetGlobalCooldown))
  (bind _returnvalue (* _abilitycd _globalcooldown))
  ;[0.13 0.7579 1] Q Ability
  (:Pressed
    (if (not (Variables|Default|GetIsDead?))
      (Utilities|FlowControl|Sequence
        (:then_0
          (Utilities|FlowControl|DoOnce false :!label _label
            (:Completed
              (Default|AbilityonCooldown (Variables|Default|GetHUDRef) _returnvalue)
              (bind _damage (CallFunction|CalculateDamage (Variables|Default|GetAttackDamage) (Variables|Default|GetCritChance) (Variables|Default|GetLifeSteal)))
              (Default|PlayerShockwave (Variables|Default|GetBPC_Attacks) (Transformation|GetWorldLocation (Variables|Default|GetCapsuleComponent)) (Utilities|Struct|MakeS_DamageInfo (* _damage 3.0) "NewEnumerator3") 5e+02 1.2e+04))))
        (:then_1
          (Utilities|FlowControl|Delay _returnvalue)
          (goto _label Reset))))))

(event Input|ActionEvents|InputActionUtility
  (params (Key :type Key%20Structure :default "None"))
  (bind _globalcooldown (Variables|Default|GetGlobalCooldown))
  (bind _utilitycd (Variables|Abilities|GetUtilityCD))
  (bind _returnvalue (* _utilitycd _globalcooldown))
  ;[0.02745 0.6549 1] Utility (roll)
  (:Pressed
    (if (not (Variables|Default|GetIsDead?))
      (Utilities|FlowControl|Sequence
        (:then_0
          (Utilities|FlowControl|DoOnce false :!label _label
            (:Completed
              (Default|UtilityonCooldown (Variables|Default|GetHUDRef) _returnvalue)
              (Utilities|DodgeRoll "/Game/DodgeRoll_Forward_Montage.DodgeRoll_Forward_Montage" "W"
                (:false
                  (Utilities|DodgeRoll "/Game/DodgeRoll_Backwards_Montage.DodgeRoll_Backwards_Montage" "S"
                    (:false
                      (Animation|Montage|PlayMontage (Variables|Character|GetMesh) "/Game/DodgeRoll_Forward_Montage.DodgeRoll_Forward_Montage") ; default if nothing is pressed
                    )))))))
        (:then_1
          (Utilities|FlowControl|Delay _returnvalue)
          (goto _label Reset))))))

(fn ConstructionScript
  (|CallParentFunction))

(fn AddSoloModifiers
  (bind _bpc_damagesystem (Variables|Default|GetBPC_DamageSystem))
  (bind _asmy_game_instance (Utilities|Casting|CastToMyGameInstance (Game|GetGameInstance)))
  (if (Variables|/Game/Blueprints/MyGameInstance.MyGameInstance_C|GetDoOnce _asmy_game_instance) ; only add modifiers on initial load
    (Variables|Default|SetAttackDamage (+ (Variables|Default|GetAttackDamage) (Variables|Character|GetAttackModifier)))
    (bind _output_get (Variables|/Game/DamageSystem/BPC_DamageSystem.BPC_DamageSystem_C|SetMaxHealth _bpc_damagesystem (+ (Variables|/Game/DamageSystem/BPC_DamageSystem.BPC_DamageSystem_C|GetMaxHealth _bpc_damagesystem) (Variables|Character|GetHealthModifier))))
    (Variables|/Game/DamageSystem/BPC_DamageSystem.BPC_DamageSystem_C|SetHealth _bpc_damagesystem _output_get)
    (Variables|/Game/Blueprints/MyGameInstance.MyGameInstance_C|SetDoOnce _asmy_game_instance false)))