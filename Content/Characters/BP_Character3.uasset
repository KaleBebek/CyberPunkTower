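; Playable Medusa character that sets up its HUD and music outside the menu and applies stat modifiers on initial load.
; Primary fire passes calculated damage to the attack component, while the cooldown-gated ability briefly slows global time, offsetting the player's time dilation and fire rate.
; Damage component events start timer-based regeneration or trigger ragdoll death, camera zoom-out and game over.
; A helper spawns per-digit Niagara damage numbers.
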(event OnDeath(BPC_DamageSystem)
  (bind _returnvalue (Game|GetPlayerController 0))
  ;[1 0.1456 0.1655] Death stuff
  (CallFunction|RagdollDeath)
  (Audio|PlaySound2D "/Game/Sounds/elevatording_Cue.elevatording_Cue" 0.2 1.0 0.0 0 0) ; dead
  (Variables|Default|SetIsDead? true)
  (Widget|RemovefromParent (Variables|Default|GetHUDRef))
  (bind _asmy_game_instance (Utilities|Casting|CastToMyGameInstance (Game|GetGameInstance)))
  (Variables|/Game/Blueprints/MyGameInstance.MyGameInstance_C|SetKilledBy _asmy_game_instance (Utilities|GetDisplayName (Variables|Default|GetDamage%20Causer)))
  (bind _zoom_out (Timeline|Timeline PlayFromStart)
    (:Update
      (Variables|/Script/Engine.SpringArmComponent|SetTargetArmLength (Variables|Default|GetCameraBoom) (Math|Float|Lerp 4e+02 7e+02 _zoom_out))
      (Utilities|FlowControl|Delay 3.0)
      (Utilities|Time|SetGlobalTimeDilation 0.0)
      (bind _returnvalue_2 (UserInterface|CreateWidget "/Game/UI_Widgets/GameOver_UI.GameOver_UI_C"))
      (UserInterface|Viewport|AddtoViewport _returnvalue_2 0)
      (Input|SetInputModeUIOnly _returnvalue 0 "DoNotLock" false)
      (Variables|/Script/Engine.PlayerController|SetbShowMouseCursor _returnvalue true)
      (Default|ResetGameDefaults _asmy_game_instance))))

(event OnDamageResponse(BPC_DamageSystem)
  (params (DamageResponse :type E_DamageResponse%20Enum :default "NewEnumerator0") (DamageCauser :type Actor%20Object%20Reference) (Amount :type Float%20%28double-precision%29) (Interuptible :type Boolean))
  ;[1 1 1] Heal over time
  (Variables|Default|SetDamage%20Causer DamageCauser)
  (CallFunction|StartHealing))

(event Custom|StartHealing
  (bind _bpc_damagesystem (Variables|Default|GetBPC_DamageSystem))
  ;[1 1 1] Heal over time
  (if (< (Variables|/Game/DamageSystem/BPC_DamageSystem.BPC_DamageSystem_C|GetHealth _bpc_damagesystem) (Variables|/Game/DamageSystem/BPC_DamageSystem.BPC_DamageSystem_C|GetMaxHealth _bpc_damagesystem))
    (bind _returnvalue (Utilities|Time|SetTimerbyFunctionName 0 "HealthRegen" 2.0 true))
    (else
      (Utilities|Time|ClearandInvalidateTimerbyHandle _returnvalue))))

(event EventBeginPlay
  ;[0.2622 1 0.2689] Player Initialization
  (|CallParentFunction)
  (if (not (Utilities|Enum|Equal(Enum) (Utilities|GetDisplayName (Game|GetGameMode)) "MenuGameMode_C_0"))
    (CallFunction|AddMedusaModifiers)
    (bind _returnvalue (UserInterface|CreateWidget "/Game/UI_Widgets/BasicHUD_UI.BasicHUD_UI_C" 0 self)) ; create this characters hud
    (bind _output_get (Variables|Default|SetHUDRef _returnvalue))
    (UserInterface|Viewport|AddtoViewport _output_get 0)
    (bind _returnvalue_2 (Audio|SpawnSound2D 0 0.05 1.0 0.0 0)) ; in game music goes here
    (Variables|Default|SetBackgroundAudio _returnvalue_2)))

(event Input|ActionEvents|InputActionPrimaryShoot
  (params (Key :type Key%20Structure :default "None"))
  ;[0.02745 0.6549 1] Primary Fire (Limits user from spam clicking before shooting again)
  (:Pressed
    (if (not (Variables|Default|GetIsDead?))
      (bind _damage (CallFunction|CalculateDamage (Variables|Default|GetAttackDamage) (Variables|Default|GetCritChance) (Variables|Default|GetLifeSteal)))
      (Default|PlayerPrimary (Variables|Default|GetBPC_Attacks) (Utilities|Struct|MakeS_DamageInfo _damage "NewEnumerator2") (Variables|Default|GetFollowCamera) (Variables|Default|GetWeapon%20Range) (Variables|Character|GetMedusaFireRate))))
  (:Released
    (Default|StopShooting (Variables|Default|GetBPC_Attacks))))

(event Input|ActionEvents|InputActionAbility
  (params (Key :type Key%20Structure :default "None"))
  (bind _abilitycd (Variables|Abilities|GetAbilityCD))
  (bind _globalcooldown (Variables|Default|GetGlobalCooldown))
  (bind _timeslowamount (Variables|Default|GetTimeSlowAmount))
  (bind _bpc_attacks (Variables|Default|GetBPC_Attacks))
  (bind _returnvalue (* _abilitycd _globalcooldown))
  (bind _returnvalue_2 (/ 1.0 _timeslowamount))
  ;[0.13 0.7579 1] Q Ability
  (:Pressed
    (if (not (Variables|Default|GetIsDead?))
      (Utilities|FlowControl|Sequence
        (:then_0
          (Utilities|FlowControl|DoOnce false :!label _label
            (:Completed
              (Default|AbilityonCooldown (Variables|Default|GetHUDRef) _returnvalue)
              (Utilities|Time|SetGlobalTimeDilation _timeslowamount)
              (Variables|Default|SetCustomTimeDilation _returnvalue_2)
              (bind _output_get (Variables|Character|SetMedusaFireRate (/ (Variables|Character|GetMedusaFireRate) _returnvalue_2)))
              (Default|UpdateFirerate _bpc_attacks _output_get)
              (Utilities|FlowControl|Delay 1.0)
              (Utilities|Time|SetGlobalTimeDilation 1.0)
              (Variables|Default|SetCustomTimeDilation 1.0)
              (bind _output_get_2 (Variables|Character|SetMedusaFireRate (Variables|Character|GetDefaultFireRate)))
              (Default|UpdateFirerate _bpc_attacks _output_get_2))))
        (:then_1
          (Utilities|FlowControl|Delay _returnvalue)
          (goto _label Reset))))))

(fn ConstructionScript
  (|CallParentFunction))

(fn MakeDamageNumbers
  (params (Location :type Vector) (DamageAmount :type Integer))
  (for _array_element (Utilities|String|GetCharacterArrayfromString (Utilities|String|ToString(Integer) DamageAmount))
    (bind _returnvalue (Niagara|SpawnSystematLocation "/Game/Niagra/FloatingNumberFX.FloatingNumberFX" Location (Math|Rotator|MakeRotator 0.0 1.8e+02 (.yaw (Pawn|GetControlRotation (Game|GetPlayerController 0) :!class /Script/Engine.Controller)))))
    (bind _output_get (LocalVariables|SetDigit%20System _returnvalue))
    (Transformation|AddLocalOffset _output_get (Math|Vector|MakeVector 0.0 (LocalVariables|GetText%20Offset) 0.0) false false)
    (LocalVariables|SetText%20Offset (+ (LocalVariables|GetText%20Offset) 25.0))
    (switch string _array_element
      (:0
        (Niagara|SetTextureObject (LocalVariables|GetDigit%20System) "user.Digit" "/Game/Images/0.0"))
      (:1
        (Niagara|SetTextureObject (LocalVariables|GetDigit%20System) "user.Digit" "/Game/Images/1.1"))
      (:2
        (Niagara|SetTextureObject (LocalVariables|GetDigit%20System) "user.Digit" "/Game/Images/2.2"))
      (:3
        (Niagara|SetTextureObject (LocalVariables|GetDigit%20System) "user.Digit" "/Game/Images/3.3"))
      (:4
        (Niagara|SetTextureObject (LocalVariables|GetDigit%20System) "user.Digit" "/Game/Images/4.4"))
      (:5
        (Niagara|SetTextureObject (LocalVariables|GetDigit%20System) "user.Digit" "/Game/Images/5.5"))
      (:6
        (Niagara|SetTextureObject (LocalVariables|GetDigit%20System) "user.Digit" "/Game/Images/6.6"))
      (:7
        (Niagara|SetTextureObject (LocalVariables|GetDigit%20System) "user.Digit" "/Game/Images/7.7"))
      (:8
        (Niagara|SetTextureObject (LocalVariables|GetDigit%20System) "user.Digit" "/Game/Images/8.8"))
      (:9
        (Niagara|SetTextureObject (LocalVariables|GetDigit%20System) "user.Digit" "/Game/Images/9.9")))))

(fn AddMedusaModifiers
  (bind _bpc_damagesystem (Variables|Default|GetBPC_DamageSystem))
  (bind _asmy_game_instance (Utilities|Casting|CastToMyGameInstance (Game|GetGameInstance)))
  (if (Variables|/Game/Blueprints/MyGameInstance.MyGameInstance_C|GetDoOnce _asmy_game_instance) ; only add modifiers on initial load
    (Variables|Default|SetAttackDamage (+ (Variables|Default|GetAttackDamage) (Variables|Character|GetAttackModifier)))
    (bind _output_get (Variables|/Game/DamageSystem/BPC_DamageSystem.BPC_DamageSystem_C|SetMaxHealth _bpc_damagesystem (+ (Variables|/Game/DamageSystem/BPC_DamageSystem.BPC_DamageSystem_C|GetMaxHealth _bpc_damagesystem) (Variables|Character|GetHealthModifier))))
    (Variables|/Game/DamageSystem/BPC_DamageSystem.BPC_DamageSystem_C|SetHealth _bpc_damagesystem _output_get)
    (Variables|/Game/Blueprints/MyGameInstance.MyGameInstance_C|SetDoOnce _asmy_game_instance false)))