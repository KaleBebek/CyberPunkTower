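; Homing explosive projectile that seeks living enemies and deals radial damage on impact, sparing BP_Character1 actors.
; After a short launch delay, a repeating loop feeds FindHomingTarget's result into ProjectileMovement as the homing target.
; The search compares distances to non-dead BP_EnemyBase actors tagged "Homing" and returns the chosen one's capsule.
; Hit destroys the hit event's own component, plays explosion effects, applies damage and draws a debug sphere.
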(event Custom|LockOn
  (bind _projectilemovement (Variables|Default|GetProjectileMovement))
  (bind _homingtarget (CallFunction|FindHomingTarget))
  (Variables|/Script/Engine.ProjectileMovementComponent|SetHomingTargetComponent _projectilemovement _homingtarget)
  (Variables|/Script/Engine.ProjectileMovementComponent|SetbIsHomingProjectile _projectilemovement true))

(event EventBeginPlay
  (Utilities|FlowControl|Delay 0.25)
  (CallFunction|Lockon :!label _label)
  (Utilities|FlowControl|Delay 0.1)
  (goto _label))

(event Collision|EventHit
  (params (MyComp :type Primitive%20Component%20Object%20Reference) (Other :type Actor%20Object%20Reference) (OtherComp :type Primitive%20Component%20Object%20Reference) (bSelfMoved :type Boolean) (HitLocation :type Vector :default "0, 0, 0") (HitNormal :type Vector :default "0, 0, 0") (NormalImpulse :type Vector :default "0, 0, 0") (Hit :type Hit%20Result%20Structure%20%28by%20ref%29))
  (Components|DestroyComponent MyComp)
  (Effects|SpawnEmitteratLocation "/Game/StarterContent/Particles/P_Explosion.P_Explosion" HitLocation)
  (Audio|PlaySoundatLocation "/Game/StarterContent/Audio/Explosion01.Explosion01" HitLocation "0, 0, 0" 0.1 1.0 0.0 0 0 0 0)
  (bind _outactors (Actor|GetAllActorsOfClass "/Game/BP_Character1.BP_Character1_C"))
  (Game|Damage|ApplyRadialDamage 25.0 HitLocation 2.5e+02 0 _outactors self 0 true "ECC_Visibility")
  (Rendering|Debug|DrawDebugSphere HitLocation 2.5e+02 12 "(R=1.000000,G=1.000000,B=1.000000,A=1.000000)" 5.0))

(fn ConstructionScript)

(fn FindHomingTarget
  (bind _outactors (Actor|GetAllActorsOfClasswithTag "/Script/Engine.Actor" "Homing"))
  (for _array_element _outactors
    (bind _asbp_enemy_base (Utilities|Casting|CastToBP_EnemyBase _array_element))
    (if (not (Variables|/Game/Enemies/BP_EnemyBase.BP_EnemyBase_C|GetIsDead? _asbp_enemy_base))
      (if (< (Math|Vector|VectorLength (Math|Vector|VectorGetAbs (- (Transformation|GetActorLocation _array_element) (Transformation|GetActorLocation)))) (Variables|Default|Getclosest%20distance))
        (Variables|Default|Setclosest%20distance (Math|Vector|VectorLength (Math|Vector|VectorGetAbs (- (Transformation|GetActorLocation _array_element) (Transformation|GetActorLocation)))))
        (Variables|Default|SetHomingTarget _array_element))))
  (if (Utilities|IsValid (Variables|Default|GetHomingTarget))
    (return (Actor|GetComponentbyClass (Variables|Default|GetHomingTarget) "/Script/Engine.CapsuleComponent"))))