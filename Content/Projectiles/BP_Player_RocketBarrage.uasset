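; Player rocket barrage projectile that flies without gravity and homes in on nearby actors tagged "Homing".
; Construction sets a pre-homing launch speed and a separate maximum speed.
; After a short delay from BeginPlay, a repeating timed loop searches tagged actors and feeds the chosen target's capsule component to ProjectileMovement.
; ClosestDistance persists between searches, so the target switches only when an actor beats the closest distance recorded so far.
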(event Custom|LockOn
  (bind _projectilemovement (Variables|Default|GetProjectileMovement))
  (bind _homingtarget (CallFunction|FindHomingTarget))
  (Variables|/Script/Engine.ProjectileMovementComponent|SetHomingTargetComponent _projectilemovement _homingtarget)
  (Variables|/Script/Engine.ProjectileMovementComponent|SetbIsHomingProjectile _projectilemovement true))

(event EventBeginPlay
  (|CallParentFunction)
  (Utilities|FlowControl|Delay 0.25)
  (CallFunction|Lockon :!label _label)
  (Utilities|FlowControl|Delay 0.1)
  (goto _label))

(fn ConstructionScript
  (bind _projectilemovement (Variables|Default|GetProjectileMovement))
  (Variables|/Script/Engine.ProjectileMovementComponent|SetInitialSpeed _projectilemovement (Variables|Default|GetSpeedBeforeHoming))
  (Variables|/Script/Engine.ProjectileMovementComponent|SetMaxSpeed _projectilemovement (Variables|Default|GetSpeed))
  (Variables|/Script/Engine.ProjectileMovementComponent|SetProjectileGravityScale _projectilemovement 0.0))

(fn FindHomingTarget
  (bind _outactors (Actor|GetAllActorsOfClasswithTag "/Script/Engine.Actor" "Homing"))
  (for _array_element _outactors
    (if (< (Math|Vector|VectorLength (Math|Vector|VectorGetAbs (- (Transformation|GetActorLocation _array_element) (Transformation|GetActorLocation)))) (Variables|Default|Getclosest%20distance))
      (Variables|Default|Setclosest%20distance (Math|Vector|VectorLength (Math|Vector|VectorGetAbs (- (Transformation|GetActorLocation _array_element) (Transformation|GetActorLocation)))))
      (Variables|Default|SetHomingTarget _array_element)))
  (if (Utilities|IsValid (Variables|Default|GetHomingTarget))
    (return (Actor|GetComponentbyClass (Variables|Default|GetHomingTarget) "/Script/Engine.CapsuleComponent"))))