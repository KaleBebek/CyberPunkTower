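; Explosive projectile that deals radial damage where it hits and destroys itself three seconds after spawning.
; On hit, it spawns explosion effects and sound, makes noise, then applies full damage in a radius at double the player character's AttackDamage, sparing all BP_Character1 actors.
; The hit then destroys only the Sphere component, leaving actor cleanup to the BeginPlay timeout.
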(event OnComponentHit(Sphere)
  (params (HitComponent :type Primitive%20Component%20Object%20Reference) (OtherActor :type Actor%20Object%20Reference) (OtherComp :type Primitive%20Component%20Object%20Reference) (NormalImpulse :type Vector :default "0, 0, 0") (Hit :type Hit%20Result%20Structure%20%28by%20ref%29)))

(event EventBeginPlay
  ;[1 1 1] Failsafe if projectile doesnt hit anything for 3 seconds it dies
  (Utilities|FlowControl|Delay 3.0)
  (Actor|DestroyActor))

(event Collision|EventActorBeginOverlap
  (params (OtherActor :type Actor%20Object%20Reference)))

(event EventTick
  (params (DeltaSeconds :type Float%20%28single-precision%29)))

(event Collision|EventHit
  (params (MyComp :type Primitive%20Component%20Object%20Reference) (Other :type Actor%20Object%20Reference) (OtherComp :type Primitive%20Component%20Object%20Reference) (bSelfMoved :type Boolean) (HitLocation :type Vector :default "0, 0, 0") (HitNormal :type Vector :default "0, 0, 0") (NormalImpulse :type Vector :default "0, 0, 0") (Hit :type Hit%20Result%20Structure%20%28by%20ref%29))
  (Effects|SpawnEmitteratLocation "/Game/StarterContent/Particles/P_Explosion.P_Explosion" HitLocation)
  (Audio|PlaySoundatLocation "/Game/StarterContent/Audio/Explosion01.Explosion01" HitLocation "0, 0, 0" 0.1 1.0 0.0 0 0 0 0)
  (Class|Actor|MakeNoise 1.0 0 HitLocation 0.0 "None")
  (bind _asbp_third_person_character (Utilities|Casting|CastToBP_ThirdPersonCharacter (Game|GetPlayerCharacter 0)))
  (bind _outactors (Actor|GetAllActorsOfClass "/Game/BP_Character1.BP_Character1_C"))
  (Game|Damage|ApplyRadialDamage (* (Variables|/Game/BP_Character1.BP_Character1_C|GetAttackDamage _asbp_third_person_character) 2.0) HitLocation 2.5e+02 0 _outactors self 0 true "ECC_Visibility")
  (Components|DestroyComponent (Variables|Default|GetSphere)))

(fn ConstructionScript)