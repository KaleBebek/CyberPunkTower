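; Spinning axe projectile Blueprint that visually rotates while it exists and removes itself after a short lifespan.
; On BeginPlay it starts SpinAxe and sets the lifespan.
; SpinAxe plays a timeline that drives only the world yaw of RotationPoint, keeping its roll and pitch, and calls itself when the timeline finishes to loop the spin.
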(event Custom|SpinAxe
  (bind _rotationpoint (Variables|Default|GetRotationPoint))
  (bind _returnvalue (Transformation|GetWorldRotation _rotationpoint))
  (bind _zrotation (Timeline|RotationTimeline PlayFromStart)
    (:Update
      (Transformation|SetWorldRotation _rotationpoint (Math|Rotator|MakeRotator (.roll _returnvalue) (.pitch _returnvalue) _zrotation) false false))
    (:Finished
      (CallFunction|SpinAxe))))

(event EventBeginPlay
  (|CallParentFunction)
  (CallFunction|SpinAxe)
  (Actor|SetLifeSpan 1.0))

(event Collision|EventActorBeginOverlap
  (params (OtherActor :type Actor%20Object%20Reference)))

(event EventTick
  (params (DeltaSeconds :type Float%20%28single-precision%29)))

(fn ConstructionScript
  (|CallParentFunction))