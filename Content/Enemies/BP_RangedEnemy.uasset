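; Ranged enemy Blueprint that roams until it spots the player, then chases and fires projectiles.
; BeginPlay calls the parent, overrides health, EXP and attack stats, and starts random roaming.
; Pawn sensing latches SeenPlayer and holds InRange through a one-second retriggerable delay, so Tick switches between stopping to shoot and chasing via AI MoveTo.
; Shooting faces the player and spawns BP_EnemyProjectile behind a delay-based cooldown.
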(event OnSeePawn(PawnSensing)
  (params (Pawn :type Pawn%20Object%20Reference))
  (Variables|Default|SetSeenPlayer? true)
  (Variables|Default|SetInRange? true)
  (Utilities|FlowControl|RetriggerableDelay 1.0)
  (Variables|Default|SetInRange? false))

(event Custom|Chase%20Player
  (Variables|/Script/Engine.CharacterMovementComponent|SetMaxWalkSpeed (Variables|Character|GetCharacterMovement) 5e+02)
  (AI|AIMoveTo self "0, 0, 0" (Game|GetPlayerCharacter 0) 1e+02 false
    (:OnSuccess
      (CallFunction|ShootPlayer))))

(event Custom|Shoot%20Player
  (bind _projectilespawnpos (Variables|Default|GetProjectileSpawnPos))
  (bind _returnvalue (Transformation|GetWorldTransform _projectilespawnpos))
  (Transformation|SetActorRotation (Math|Rotator|FindRelativeLookatRotation (Math|Conversions|ToTransform(Vector) (Transformation|GetActorLocation)) (Transformation|GetActorLocation (Game|GetPlayerCharacter 0))))
  (if (Variables|Default|GetCanAttack?)
    (Game|SpawnActorfromClass "/Game/Projectiles/BP_EnemyProjectile.BP_EnemyProjectile_C" (Math|Transform|MakeTransform (.location _returnvalue) (.rotation _returnvalue) "0.250000,0.250000,0.250000") "Undefined" 0 0)
    (Variables|Default|SetCanAttack? false)
    (Utilities|FlowControl|Delay 1.0) ; Shoot Delay
    (Variables|Default|SetCanAttack? true)))

(event EventBeginPlay
  ;[1 1 1] Set stats of this enemy
  (|CallParentFunction)
  (bind _output_get (Variables|Default|SetMaxHealth 5e+01))
  (Variables|Default|SetHealth _output_get)
  (Variables|Default|SetEXP%20Value 5)
  (Variables|Default|SetAttack 5.0)
  (CallFunction|RandomRoam))

(event EventTick
  (params (DeltaSeconds :type Float%20%28single-precision%29))
  (CallFunction|UpdateHealthBar)
  (if (not (Variables|Default|GetIsDead?))
    (if (Variables|Default|GetSeenPlayer?)
      (if (Variables|Default|GetInRange?)
        (Class|NavMovementComponent|StopActiveMovement (Variables|Character|GetCharacterMovement))
        (CallFunction|ShootPlayer)
        (else
          (CallFunction|ChasePlayer))))))

(fn ConstructionScript)