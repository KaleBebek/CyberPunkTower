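; Base enemy character that registers with the game mode's enemy count, roams random reachable points and damages the player through a left-foot sphere trace.
; Taking damage flags the player as seen, reduces health, reveals the health bar widget and spawns floating damage numbers, one Niagara system per textured digit.
; Death awards EXP, decrements the count, disables selected collision, plays an animation before despawning, and opens the elevator door for bosses.
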(event Custom|Random%20Roam
  (AI|AIMoveTo self (.RandomLocation (AI|Navigation|GetRandomReachablePointinRadius (Transformation|GetActorLocation) 2.5e+03 0 0)) 0 5.0 false
    (:OnSuccess
      (Utilities|FlowControl|Delay (Math|Random|RandomFloatinRange 0.5 5.0)))
    (:OnFail
      _))
  (CallFunction|RandomRoam))

(event EventTick
  (params (DeltaSeconds :type Float%20%28single-precision%29))
  (if (Variables|Default|GetHunting?)
    (Variables|Default|SetSeenPlayer? true)))

(event Game|Damage|EventAnyDamage
  (params (Damage :type Float%20%28single-precision%29) (DamageType :type Damage%20Type%20Object%20Reference) (InstigatedBy :type Controller%20Object%20Reference) (DamageCauser :type Actor%20Object%20Reference))
  (bind _returnvalue (Transformation|GetActorLocation))
  (if (not (Variables|Default|GetIsDead?))
    (Rendering|SetVisibility (Variables|Default|GetHealth%20Bar%20Widget) true false)
    (CallFunction|MakeDamageNumbers (Math|Vector|MakeVector (.x _returnvalue) (+ (.y _returnvalue) (Math|Random|RandomFloatinRange -5e+01 5e+01)) (+ (.z _returnvalue) 1.2e+02)) (Math|Float|Truncate Damage))
    (Variables|Default|SetSeenPlayer? true)
    (bind _output_get (Variables|Default|SetHealth (Math|Float|Clamp(Float) (- (Variables|Default|GetHealth) Damage) 0.0 (Variables|Default|GetMaxHealth))))
    (if (== _output_get 0.0)
      (Variables|Default|SetIsDead? true)
      (CallFunction|Death))))

(event EventBeginPlay
  (bind _asbp_third_person_game_mode (Utilities|Casting|CastToBP_ThirdPersonGameMode (Game|GetGameMode)))
  (Variables|/Game/BP_ThirdPersonGameMode.BP_ThirdPersonGameMode_C|SetEnemies%20Remaining _asbp_third_person_game_mode (+ (Variables|/Game/BP_ThirdPersonGameMode.BP_ThirdPersonGameMode_C|GetEnemies%20Remaining _asbp_third_person_game_mode) 1)))

(fn ConstructionScript)

(fn HitDetect
  (bind _mesh (Variables|Character|GetMesh))
  (bind _returnvalue (Transformation|GetSocketLocation _mesh "foot_l"))
  (bind _outhit (Collision|SphereTraceForObjects _returnvalue _returnvalue 5e+01 (Variables|Default|GetObject%20Types) false 0 "ForDuration"))
  (bind _asbp_third_person_character (Utilities|Casting|CastToBP_ThirdPersonCharacter (.HitActor (Collision|BreakHitResult _outhit))))
  (Game|Damage|ApplyDamage _asbp_third_person_character (* (Variables|Default|GetAttack) 1.0) 0 self))

(fn UpdateHealthBar
  (bind _aswb_enemy_hpbar (Utilities|Casting|CastToWB_EnemyHPBar (UserInterface|GetWidget (Variables|Default|GetHealth%20Bar%20Widget))))
  (Progress|SetPercent (Variables|/Game/UI_Widgets/WB_EnemyHPBar.WB_EnemyHPBar_C|GetEnemyHealthBar _aswb_enemy_hpbar) (/ (Variables|Default|GetHealth) (Variables|Default|GetMaxHealth)))
  (Transformation|SetWorldRotation (Variables|Default|GetHealth%20Bar%20Widget) (Math|Rotator|FindLookatRotation (Transformation|GetWorldLocation (Variables|Default|GetHealth%20Bar%20Widget)) (Transformation|GetActorLocation (Game|GetPlayerCameraManager 0))) false false))

(fn Death
  (Rendering|SetVisibility (Variables|Default|GetHealth%20Bar%20Widget) false false)
  (bind _asbp_third_person_character (Utilities|Casting|CastToBP_ThirdPersonCharacter (Game|GetPlayerCharacter 0)))
  (Default|AddEXP _asbp_third_person_character (Variables|Default|GetEXP%20Value))
  (bind _asbp_third_person_game_mode (Utilities|Casting|CastToBP_ThirdPersonGameMode (Game|GetGameMode)))
  (Variables|/Game/BP_ThirdPersonGameMode.BP_ThirdPersonGameMode_C|SetEnemies%20Remaining _asbp_third_person_game_mode (- (Variables|/Game/BP_ThirdPersonGameMode.BP_ThirdPersonGameMode_C|GetEnemies%20Remaining _asbp_third_person_game_mode) 1))
  (Components|Movement|StopMovementImmediately (Variables|Character|GetCharacterMovement))
  (for _array_element (Variables|Default|GetArray)
    (Collision|SetCollisionResponsetoChannel (Variables|Collision|GetCapsuleComponent) _array_element "ECR_Ignore")
    (Components|Animation|PlayAnimation (Variables|Character|GetMesh) "/Game/Death_1.Death_1" false)
    (Actor|SetLifeSpan 2.0)
    (if (Variables|Default|GetIsBoss?)
      (bind _returnvalue (Actor|GetActorOfClass "/Game/Blueprints/DoubleElevatorDoor.DoubleElevatorDoor_C"))
      (Default|OpenElevator _returnvalue))))

(fn MakeDamageNumbers
  (params (Location :type Vector) (DamageAmount :type Integer))
  (for _array_element (Utilities|String|GetCharacterArrayfromString (Utilities|String|ToString(Integer) DamageAmount))
    (bind _returnvalue (Niagara|SpawnSystematLocation "/Game/FloatingNumberFX.FloatingNumberFX" Location (Math|Rotator|MakeRotator 0.0 1.8e+02 (.yaw (Pawn|GetControlRotation (Game|GetPlayerController 0) :!class /Script/Engine.Controller)))))
    (bind _output_get (LocalVariables|SetDigit%20System _returnvalue))
    (Transformation|AddLocalOffset _output_get (Math|Vector|MakeVector 0.0 (LocalVariables|GetText%20Offset) 0.0) false false)
    (LocalVariables|SetText%20Offset (+ (LocalVariables|GetText%20Offset) 25.0))
    (switch string _array_element
      (:0
        (Niagara|SetTextureObject (LocalVariables|GetDigit%20System) "user.Digit" "/Game/Textures/0.0"))
      (:1
        (Niagara|SetTextureObject (LocalVariables|GetDigit%20System) "user.Digit" "/Game/Textures/1.1"))
      (:2
        (Niagara|SetTextureObject (LocalVariables|GetDigit%20System) "user.Digit" "/Game/Textures/2.2"))
      (:3
        (Niagara|SetTextureObject (LocalVariables|GetDigit%20System) "user.Digit" "/Game/Textures/3.3"))
      (:4
        (Niagara|SetTextureObject (LocalVariables|GetDigit%20System) "user.Digit" "/Game/Textures/4.4"))
      (:5
        (Niagara|SetTextureObject (LocalVariables|GetDigit%20System) "user.Digit" "/Game/Textures/5.5"))
      (:6
        (Niagara|SetTextureObject (LocalVariables|GetDigit%20System) "user.Digit" "/Game/Textures/6.6"))
      (:7
        (Niagara|SetTextureObject (LocalVariables|GetDigit%20System) "user.Digit" "/Game/Textures/7.7"))
      (:8
        (Niagara|SetTextureObject (LocalVariables|GetDigit%20System) "user.Digit" "/Game/Textures/8.8"))
      (:9
        (Niagara|SetTextureObject (LocalVariables|GetDigit%20System) "user.Digit" "/Game/Textures/9.9")))))