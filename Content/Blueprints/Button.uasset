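; An interactable button that alerts enemies and calls the elevator on a 30-second countdown.
; A box overlap with the player shows or hides an interact prompt widget.
; Interact fires once, playing a sound, showing an ElevatorTimer widget and setting SeenPlayer on every BP_EnemyBase.
; The delay sits inside that enemy loop, then removes the timer and opens Elevator_BP if it is closed.
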(event OnComponentBeginOverlap(Box)
  (params (OverlappedComponent :type Primitive%20Component%20Object%20Reference) (OtherActor :type Actor%20Object%20Reference) (OtherComp :type Primitive%20Component%20Object%20Reference) (OtherBodyIndex :type Integer) (bFromSweep :type Boolean) (SweepResult :type Hit%20Result%20Structure%20%28by%20ref%29))
  (if (== OtherActor (Game|GetPlayerCharacter 0))
    (UserInterface|Viewport|AddtoViewport (Variables|Default|Getinteract%20prompt) 0)))

(event OnComponentEndOverlap(Box)
  (params (OverlappedComponent :type Primitive%20Component%20Object%20Reference) (OtherActor :type Actor%20Object%20Reference) (OtherComp :type Primitive%20Component%20Object%20Reference) (OtherBodyIndex :type Integer))
  (if (== (Game|GetPlayerCharacter 0) OtherActor)
    (Widget|RemovefromParent (Variables|Default|Getinteract%20prompt))))

(event EventInteract
  (Utilities|FlowControl|DoOnce false
    (:Completed
      ;[1 1 1] Alert enemies
      (Audio|PlaySound2D "/Game/Sounds/Cyberpunk_game_Cue.Cyberpunk_game_Cue" 0.2 1.0 0.0 0 0)
      (bind _returnvalue (UserInterface|CreateWidget "/Game/ElevatorTimer.ElevatorTimer_C"))
      (UserInterface|Viewport|AddtoViewport _returnvalue 0)
      (bind _outactors (Actor|GetAllActorsOfClass "/Game/Enemies/BP_EnemyBase.BP_EnemyBase_C"))
      (for _array_element _outactors
        (Variables|/Game/Enemies/BP_EnemyBase.BP_EnemyBase_C|SetSeenPlayer? _array_element true)
        (Utilities|FlowControl|Delay 3e+01) ; elevator timer (also set in widget)
        (Widget|RemovefromParent _returnvalue)
        (bind _returnvalue_2 (Actor|GetActorOfClass "/Game/Elevator_BP.Elevator_BP_C"))
        (if (not (Variables|/Game/Elevator_BP.Elevator_BP_C|GetIsOpen? _returnvalue_2))
          (Default|OpenElevator _returnvalue_2))))))

(event Collision|EventActorBeginOverlap
  (params (OtherActor :type Actor%20Object%20Reference)))

(event EventTick
  (params (DeltaSeconds :type Float%20%28single-precision%29)))

(event EventBeginPlay
  (bind _returnvalue (UserInterface|CreateWidget "/Game/UI_Widgets/p_interact.p_interact_C"))
  (Variables|Default|Setinteract%20prompt _returnvalue))

(fn ConstructionScript)