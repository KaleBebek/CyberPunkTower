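; Game instance that holds run state for a floor-based combat game, with a function to restore it to a fresh start.
; ResetGameDefaults sets floor progress, the global ability cooldown, character level, experience and combat stats back to starting values.
; It also clears enemy count, kill and damage tallies and re-arms a DoOnce flag.
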(fn ResetGameDefaults
  (Variables|Default|SetFloor 1)
  (Variables|Default|SetEnemyCount 0)
  (Variables|Default|SetGlobalAbilityCD 1.0)
  (Variables|CharacterStats|SetCharacterLevel 1)
  (Variables|CharacterStats|SetCharacterEXP 0)
  (Variables|CharacterStats|SetCharacterEXPNeeded 100)
  (Variables|CharacterStats|SetCharacterMaxHP 1e+02)
  (Variables|CharacterStats|SetCharacterAttack 5.0)
  (Variables|CharacterStats|SetCharacterCritChance 0.0)
  (Variables|CharacterStats|SetCharacterFireRate 0.25)
  (Variables|CharacterStats|SetCharacterLifeSteal 0.0)
  (Variables|Default|SetTotalEnemiesKilled 0)
  (Variables|Default|SetTotalDamageDealt 0)
  (Variables|Default|SetEnemiesKilledPerFloor 0)
  (Variables|Default|SetDoOnce true))