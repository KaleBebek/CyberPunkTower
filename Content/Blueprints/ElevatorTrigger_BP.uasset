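; Elevator trigger that ends a floor: on any actor overlap it disables player input, walks the player to the elevator center and eases their view rotation via a timeline.
; Each timeline update destroys all enemies, closes the exit, saves player stats to the game instance and resets the kill count.
; A DoOnce then increments the floor, plays the rise sound, updates floor displays and loads the next map, switching to BossMap on floor five.
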(event EventBeginPlay)

(event Collision|EventActorBeginOverlap
  (params (OtherActor :type Actor%20Object%20Reference))
  (bind _returnvalue (Game|GetPlayerController 0))
  (bind _returnvalue_2 (Actor|GetActorOfClass "/Game/CenterOfElevator_BP.CenterOfElevator_BP_C"))
  (Input|DisableInput (Game|GetPlayerCharacter 0) _returnvalue)
  (AI|Navigation|SimpleMovetoActor _returnvalue _returnvalue_2)
  (bind _rotateplayerorientation (Timeline|RotateToCenter PlayFromStart)
    (:Update
      (Pawn|SetControlRotation _returnvalue (Math|Rotator|Lerp(Rotator) (Pawn|GetControlRotation _returnvalue :!class /Script/Engine.Controller) "0, 0, 0" _rotateplayerorientation true))
      (bind _outactors (Actor|GetAllActorsOfClass "/Game/EnemiesRevamped/BP_Enemy_Base.BP_Enemy_Base_C"))
      ;[1 1 1] temporary kill every enemy
      (for _array_element _outactors
        (Actor|DestroyActor _array_element))
      (bind _returnvalue_3 (Actor|GetActorOfClass "/Game/Blueprints/ElevatorExit.ElevatorExit_C"))
      (Default|CloseElevator _returnvalue_3)
      (bind _asmy_game_instance (Utilities|Casting|CastToMyGameInstance (Game|GetGameInstance)))
      (bind _output_get (Variables|Default|SetGame%20Instance%20Ref _asmy_game_instance))
      (bind _asbp_third_person_character (Utilities|Casting|CastToBP_ThirdPersonCharacter (Game|GetPlayerCharacter 0)))
      (Variables|Default|SetDamage%20System%20Ref (Variables|/Game/Characters/BP_ThirdPersonCharacter.BP_ThirdPersonCharacter_C|GetBPC_DamageSystem _asbp_third_person_character))
      (CallFunction|SavePlayerStats)
      (CallFunction|ClearEnemyKills)
      (Utilities|FlowControl|DoOnce false
        (:Completed
          (bind _output_get_2 (Variables|/Game/Blueprints/MyGameInstance.MyGameInstance_C|SetFloor _output_get (+ (Variables|/Game/Blueprints/MyGameInstance.MyGameInstance_C|GetFloor _output_get) 1))) ; increase stage once enter elevator
          (Utilities|FlowControl|Delay 2.0)
          (Audio|PlaySound2D "/Game/Sounds/ElevatorRise.ElevatorRise" 0.5 1.0 0.0 0 0)
          (bind _outactors_2 (Actor|GetAllActorsOfClass "/Game/Blueprints/FloorDisplay.FloorDisplay_C"))
          (Utilities|FlowControl|Delay 0.5)
          (Default|UpdateFloor _outactors_2 _output_get_2)
          (Utilities|FlowControl|Delay 1.5)
          (if (== _output_get_2 5)
            (Game|OpenLevel(byName) "BossMap")
            (else
              (Game|OpenLevel(byName) "ThirdPersonMap"))))))))

(fn ConstructionScript)

(fn SavePlayerStats
  (bind _game_instance_ref (Variables|Default|GetGame%20Instance%20Ref))
  (bind _returnvalue (Actor|GetActorOfClass "/Game/Characters/BP_ThirdPersonCharacter.BP_ThirdPersonCharacter_C"))
  (Variables|/Game/Blueprints/MyGameInstance.MyGameInstance_C|SetCharacterMaxHP _game_instance_ref (Variables|/Game/DamageSystem/BPC_DamageSystem.BPC_DamageSystem_C|GetMaxHealth (Variables|Default|GetDamage%20System%20Ref)))
  (Variables|/Game/Blueprints/MyGameInstance.MyGameInstance_C|SetCharacterAttack _game_instance_ref (Variables|/Game/Characters/BP_ThirdPersonCharacter.BP_ThirdPersonCharacter_C|GetAttackDamage _returnvalue))
  (Variables|/Game/Blueprints/MyGameInstance.MyGameInstance_C|SetGlobalAbilityCD _game_instance_ref (Variables|/Game/Characters/BP_ThirdPersonCharacter.BP_ThirdPersonCharacter_C|GetGlobalCooldown _returnvalue))
  (Variables|/Game/Blueprints/MyGameInstance.MyGameInstance_C|SetCharacterFireRate _game_instance_ref (Variables|/Game/Characters/BP_ThirdPersonCharacter.BP_ThirdPersonCharacter_C|GetFire%20Rate _returnvalue)))

(fn ClearEnemyKills
  (Variables|/Game/Blueprints/MyGameInstance.MyGameInstance_C|SetEnemiesKilledPerFloor (Variables|Default|GetGame%20Instance%20Ref) 0))