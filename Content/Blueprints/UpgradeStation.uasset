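; UpgradeStation is a single-use interactable that sells the player an upgrade for credits.
; A Box overlap shows or hides an interact prompt widget for the player character until the station is used.
; Interact checks the character's TotalCredits against a fixed cost, calls PickUpgrade, and deducts the credits.
; A successful purchase marks it used, swaps the button material, hides the point light and removes the prompt, while failures only print messages.
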(event OnComponentBeginOverlap(Box)
  (params (OverlappedComponent :type Primitive%20Component%20Object%20Reference) (OtherActor :type Actor%20Object%20Reference) (OtherComp :type Primitive%20Component%20Object%20Reference) (OtherBodyIndex :type Integer) (bFromSweep :type Boolean) (SweepResult :type Hit%20Result%20Structure%20%28by%20ref%29))
  (if (not (Variables|Default|GetUsed?))
    (if (== OtherActor (Game|GetPlayerCharacter 0))
      (UserInterface|Viewport|AddtoViewport (Variables|Default|GetInteractPrompt) 0))))

(event OnComponentEndOverlap(Box)
  (params (OverlappedComponent :type Primitive%20Component%20Object%20Reference) (OtherActor :type Actor%20Object%20Reference) (OtherComp :type Primitive%20Component%20Object%20Reference) (OtherBodyIndex :type Integer))
  (if (== (Game|GetPlayerCharacter 0) OtherActor)
    (Widget|RemovefromParent (Variables|Default|GetInteractPrompt))))

(event EventInteract
  (bind _asbp_third_person_character (Utilities|Casting|CastToBP_ThirdPersonCharacter (Game|GetPlayerCharacter 0)))
  (if (Variables|Default|GetUsed?)
    (Development|PrintString "already used")
    (elif (>= (Variables|/Game/Characters/BP_ThirdPersonCharacter.BP_ThirdPersonCharacter_C|GetTotalCredits _asbp_third_person_character) (Variables|Default|GetCreditsRequired))
      (Variables|Default|SetUsed? true)
      (Default|PickUpgrade _asbp_third_person_character)
      (Variables|/Game/Characters/BP_ThirdPersonCharacter.BP_ThirdPersonCharacter_C|SetTotalCredits _asbp_third_person_character (- (Variables|/Game/Characters/BP_ThirdPersonCharacter.BP_ThirdPersonCharacter_C|GetTotalCredits _asbp_third_person_character) (Variables|Default|GetCreditsRequired)))
      (Rendering|Material|SetMaterial (Variables|Default|Getbutton) 0 "/Game/StarterContent/Materials/M_Glass.M_Glass")
      (Rendering|SetVisibility (Variables|Default|GetPointLight) false false)
      (Widget|RemovefromParent (Variables|Default|GetInteractPrompt))
      (else
        (Development|PrintString "not enough credits")))))

(event EventBeginPlay
  (bind _returnvalue (UserInterface|CreateWidget "/Game/UI_Widgets/UpgradeStationInteract_UI.UpgradeStationInteract_UI_C"))
  (Variables|Default|SetInteractPrompt _returnvalue)
  (Variables|Default|SetCreditsRequired 21))

(fn ConstructionScript)