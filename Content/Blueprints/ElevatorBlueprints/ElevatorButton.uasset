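; ElevatorButton is an interactable actor that spends the player's keycard to trigger the elevator exit sequence.
; Its box overlap shows or removes an interact prompt widget for the player.
; On Interact with a keycard, a one-time branch collapses the prompt and checks the game mode's remaining enemies.
; If any remain, it shows an ElevatorTimer widget and sets all enemies attacking the player; otherwise it opens the ElevatorExit.
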(event OnComponentBeginOverlap(Box)
  (params (OverlappedComponent :type Primitive%20Component%20Object%20Reference) (OtherActor :type Actor%20Object%20Reference) (OtherComp :type Primitive%20Component%20Object%20Reference) (OtherBodyIndex :type Integer) (bFromSweep :type Boolean) (SweepResult :type Hit%20Result%20Structure%20%28by%20ref%29))
  (if (== OtherActor (Game|GetPlayerCharacter 0))
    (UserInterface|Viewport|AddtoViewport (Variables|Default|Getinteract%20prompt) 0)))

(event OnComponentEndOverlap(Box)
  (params (OverlappedComponent :type Primitive%20Component%20Object%20Reference) (OtherActor :type Actor%20Object%20Reference) (OtherComp :type Primitive%20Component%20Object%20Reference) (OtherBodyIndex :type Integer))
  (if (== (Game|GetPlayerCharacter 0) OtherActor)
    (Widget|RemovefromParent (Variables|Default|Getinteract%20prompt))))

(event EventInteract
  ;[1 1 1] Start countdown if you have keycard
  (bind _asbp_third_person_character (Utilities|Casting|CastToBP_ThirdPersonCharacter (Game|GetPlayerCharacter 0)))
  (if (Variables|/Game/Characters/BP_ThirdPersonCharacter.BP_ThirdPersonCharacter_C|GetAquiredKeycard _asbp_third_person_character)
    (Variables|/Game/Characters/BP_ThirdPersonCharacter.BP_ThirdPersonCharacter_C|SetAquiredKeycard _asbp_third_person_character false) ; used up keycard
    (Utilities|FlowControl|DoOnce false
      (:Completed
        (Widget|SetVisibility (Variables|Default|Getinteract%20prompt) "Collapsed")
        (bind _asbp_third_person_game_mode (Utilities|Casting|CastToBP_ThirdPersonGameMode (Game|GetGameMode)))
        (if (> (Variables|/Game/BP_ThirdPersonGameMode.BP_ThirdPersonGameMode_C|GetEnemies%20Remaining _asbp_third_person_game_mode) 0) ; true if enemies are left, otherwise just open door
          (bind _returnvalue (UserInterface|CreateWidget "/Game/Blueprints/ElevatorBlueprints/ElevatorTimer.ElevatorTimer_C"))
          (UserInterface|Viewport|AddtoViewport _returnvalue 0)
          (bind _outactors (Actor|GetAllActorsOfClass "/Game/EnemiesRevamped/BP_Enemy_Base.BP_Enemy_Base_C"))
          (for _array_element _outactors
            (Default|SetStateasAttacking (Variables|/Game/EnemiesRevamped/BP_Enemy_Base.BP_Enemy_Base_C|GetAIC_Enemy_Base _array_element) (Game|GetPlayerCharacter 0) false))
          (else
            (bind _returnvalue_2 (Actor|GetActorOfClass "/Game/Blueprints/ElevatorBlueprints/ElevatorExit.ElevatorExit_C"))
            (if (not (Variables|/Game/Blueprints/ElevatorBlueprints/ElevatorExit.ElevatorExit_C|GetIsOpen? _returnvalue_2))
              (Default|OpenElevator _returnvalue_2))))))))

(event Collision|EventActorBeginOverlap
  (params (OtherActor :type Actor%20Object%20Reference)))

(event EventTick
  (params (DeltaSeconds :type Float%20%28single-precision%29)))

(event EventBeginPlay
  (bind _returnvalue (UserInterface|CreateWidget "/Game/UI_Widgets/ElevatorBtn_Interact.ElevatorBtn_Interact_C"))
  (Variables|Default|Setinteract%20prompt _returnvalue))

(fn ConstructionScript)