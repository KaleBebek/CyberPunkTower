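; ElevatorExit is an elevator exit Blueprint whose two sliding door cubes open and close.
; OpenElevator sets IsOpen, plays a 2D ding and runs a timeline that lerps both cubes' relative locations from their Current to New positions.
; CloseElevator runs a separate timeline that lerps them back, without clearing IsOpen or playing a sound.
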(event Custom|CloseElevator
  (bind _slidedoors (Timeline|CloseDoors PlayFromStart)
    (:Update
      (Transformation|SetRelativeLocation (Variables|Default|GetCubeLeft) (Math|Vector|Lerp(Vector) (Variables|Default|GetNewLeft) (Variables|Default|GetCurrentLeft) _slidedoors) false false)
      (Transformation|SetRelativeLocation (Variables|Default|GetCubeRight) (Math|Vector|Lerp(Vector) (Variables|Default|GetNewRight) (Variables|Default|GetCurrentRight) _slidedoors) false false))))

(event Custom|OpenElevator
  (Variables|Default|SetIsOpen? true)
  (Audio|PlaySound2D "/Game/Sounds/Elevator_Ding.Elevator_Ding" 0.5 1.0 0.0 0 0)
  (bind _slidedoors (Timeline|OpenDoors PlayFromStart)
    (:Update
      (Transformation|SetRelativeLocation (Variables|Default|GetCubeLeft) (Math|Vector|Lerp(Vector) (Variables|Default|GetCurrentLeft) (Variables|Default|GetNewLeft) _slidedoors) false false)
      (Transformation|SetRelativeLocation (Variables|Default|GetCubeRight) (Math|Vector|Lerp(Vector) (Variables|Default|GetCurrentRight) (Variables|Default|GetNewRight) _slidedoors) false false))))

(fn ConstructionScript)