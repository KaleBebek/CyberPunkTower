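; MusicBox is a Blueprint that controls background music through custom events to play, stop, pause and resume it.
; PlayMusic spawns a 2D sound, stores it in the Music variable and fades it in, without stopping any previously stored sound.
; StopMusic fades that stored audio component out, while pause and resume toggle its paused state, each only when the reference is valid.
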(event Custom|PlayMusic
  (params (Sound :type Sound%20Base%20Object%20Reference) (VolumeMultiplier :type Float%20%28single-precision%29) (FadeInDuration :type Float%20%28single-precision%29))
  (bind _returnvalue (Audio|SpawnSound2D Sound VolumeMultiplier 1.0 0.0 0))
  (bind _output_get (Variables|Default|SetMusic _returnvalue))
  (Audio|Components|Audio|FadeIn _output_get FadeInDuration 1.0 0.0 "Linear" :!class /Script/Engine.AudioComponent))

(event Custom|StopMusic
  (params (FadeOutDuration :type Float%20%28single-precision%29))
  (bind _music (Variables|Default|GetMusic)
    (:then
      (Audio|Components|Audio|FadeOut _music FadeOutDuration 0.0 "Linear" :!class /Script/Engine.AudioComponent))
    (:else)))

(event Custom|PauseMusic
  (bind _music (Variables|Default|GetMusic)
    (:then
      (Class|AudioComponent|SetPaused _music true))
    (:else)))

(event Custom|ResumeMusic
  (bind _music (Variables|Default|GetMusic)
    (:then
      (Class|AudioComponent|SetPaused _music false))
    (:else)))

(event EventBeginPlay)

(fn ConstructionScript)