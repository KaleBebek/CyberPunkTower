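; Double elevator door actor that slides two panels open when its OpenElevator event is called.
; The event sets IsOpen, plays a quiet 2D ding, and starts the OpenDoors timeline from the beginning.
; The timeline's SlideDoors track drives a lerp of each cube's relative location from its current to its new position, without sweeping.
; The graph contains no closing logic.
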(event Custom|OpenElevator
  (Variables|Default|SetIsOpen? true)
  (Audio|PlaySound2D "/Game/Sounds/elevatording_Cue.elevatording_Cue" 0.2 1.0 0.0 0 0)
  (bind _slidedoors (Timeline|OpenDoors PlayFromStart)
    (:Update
      (Transformation|SetRelativeLocation (Variables|Default|GetCubeLeft) (Math|Vector|Lerp(Vector) (Variables|Default|GetCurrentLeft) (Variables|Default|GetNewLeft) _slidedoors) false false)
      (Transformation|SetRelativeLocation (Variables|Default|GetCubeRight) (Math|Vector|Lerp(Vector) (Variables|Default|GetCurrentRight) (Variables|Default|GetNewRight) _slidedoors) false false))))

(event EventBeginPlay)

(event Collision|EventActorBeginOverlap
  (params (OtherActor :type Actor%20Object%20Reference)))

(event EventTick
  (params (DeltaSeconds :type Float%20%28single-precision%29)))

(fn ConstructionScript)