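; Exit elevator Blueprint with two sliding door meshes that open and close through OpenElevator and CloseElevator events.
; Opening sets IsOpen, plays a quiet 2D ding and runs a timeline that lerps both doors from their current to new relative locations.
; Closing clears IsOpen and runs a separate timeline that lerps them back, without a sound.
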(event Custom|CloseElevator
  (Variables|Default|SetIsOpen? false)
  (bind _slidedoors (Timeline|Timeline PlayFromStart)
    (:Update
      (Transformation|SetRelativeLocation (Variables|Default|GetCubeLeft) (Math|Vector|Lerp(Vector) (Variables|Default|GetNewLeft) (Variables|Default|GetCurrentLeft) _slidedoors) false false)
      (Transformation|SetRelativeLocation (Variables|Default|GetCubeRight) (Math|Vector|Lerp(Vector) (Variables|Default|GetNewRight) (Variables|Default|GetCurrentRight) _slidedoors) false false))))

(event Custom|OpenElevator
  (Variables|Default|SetIsOpen? true)
  (Audio|PlaySound2D "/Game/Sounds/elevatording_Cue.elevatording_Cue" 0.2 1.0 0.0 0 0)
  (bind _slidedoors (Timeline|OpenDoors PlayFromStart)
    (:Update
      (Transformation|SetRelativeLocation (Variables|Default|GetCubeLeft) (Math|Vector|Lerp(Vector) (Variables|Default|GetCurrentLeft) (Variables|Default|GetNewLeft) _slidedoors) false false)
      (Transformation|SetRelativeLocation (Variables|Default|GetCubeRight) (Math|Vector|Lerp(Vector) (Variables|Default|GetCurrentRight) (Variables|Default|GetNewRight) _slidedoors) false false))))

(fn ConstructionScript)