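; BP_EnemyBase is an enemy base class providing health, death, random roaming and a melee hit check against the player.
; AnyDamage flags SeenPlayer, lowers clamped Health and destroys the actor at zero.
; RandomRoam uses AIMoveTo toward random reachable points, repeating after a short delay only on success.
; HitDetect sphere-traces at the foot_l socket with debug drawing and damages BP_MainCharacter1; nothing here calls it or starts roaming.
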(event Custom|Random%20Roam
  (AI|AIMoveTo self (.RandomLocation (AI|Navigation|GetRandomReachablePointinRadius (Transformation|GetActorLocation) 2.5e+03 0 0)) 0 5.0 false
    (:OnSuccess
      (Utilities|FlowControl|Delay 1.0)
      (CallFunction|RandomRoam))))

(event EventBeginPlay)

(event Collision|EventActorBeginOverlap
  (params (OtherActor :type Actor%20Object%20Reference)))

(event EventTick
  (params (DeltaSeconds :type Float%20%28single-precision%29)))

(event Game|Damage|EventAnyDamage
  (params (Damage :type Float%20%28single-precision%29) (DamageType :type Damage%20Type%20Object%20Reference) (InstigatedBy :type Controller%20Object%20Reference) (DamageCauser :type Actor%20Object%20Reference))
  (if (not (Variables|Default|GetIsDead?))
    (Variables|Default|SetSeenPlayer? true)
    (bind _output_get (Variables|Default|SetHealth (Math|Float|Clamp(Float) (- (Variables|Default|GetHealth) Damage) 0.0 (Variables|Default|GetMaxHealth))))
    (if (== _output_get 0.0)
      (Variables|Default|SetIsDead? true)
      (Actor|DestroyActor))))

(fn ConstructionScript)

(fn HitDetect
  (bind _mesh (Variables|Character|GetMesh))
  (bind _returnvalue (Transformation|GetSocketLocation _mesh "foot_l"))
  (bind _outhit (Collision|SphereTraceForObjects _returnvalue _returnvalue 5e+01 (Variables|Default|GetObject%20Types) false 0 "ForDuration"))
  (bind _asbp_main_character_1 (Utilities|Casting|CastToBP_MainCharacter1 (.HitActor (Collision|BreakHitResult _outhit))))
  (Game|Damage|ApplyDamage _asbp_main_character_1 1.0 0 self))