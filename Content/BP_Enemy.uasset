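; BP_Enemy is a melee enemy that chases the player once its pawn sensing sees a pawn, then kicks.
; BeginPlay sets health and calls RandomRoam; a sighting permanently sets SeenPlayer.
; Tick then either re-issues an AI move toward the player at raised speed or halts movement during attacks.
; Reaching the player plays a kick montage, whose returned length times the delay before attacking again.
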(event OnSeePawn(PawnSensing)
  (params (Pawn :type Pawn%20Object%20Reference))
  (Variables|Default|SetSeenPlayer? true))

(event Custom|Chase%20Player
  (if (Variables|Default|GetSeenPlayer?)
    (Variables|/Script/Engine.CharacterMovementComponent|SetMaxWalkSpeed (Variables|Character|GetCharacterMovement) 5e+02)
    (AI|AIMoveTo self "0, 0, 0" (Game|GetPlayerCharacter 0) 5e+01 false
      (:OnSuccess
        (CallFunction|AttackPlayer)))))

(event Custom|Attack%20Player
  (if (Variables|Default|GetCanAttack?)
    (Variables|Default|SetIsAttacking? true)
    (Variables|Default|SetCanAttack? false)
    (bind _returnvalue (Animation|PlayAnimMontage "/Game/EnemyKickMontage.EnemyKickMontage" 1.0 "None"))
    (Utilities|FlowControl|Delay _returnvalue)
    (Variables|Default|SetCanAttack? true)
    (Variables|Default|SetIsAttacking? false)))

(event EventBeginPlay
  ;[1 1 1] Set stats of this enemy
  (bind _output_get (Variables|Default|SetMaxHealth 1e+02))
  (Variables|Default|SetHealth _output_get)
  (CallFunction|RandomRoam))

(event EventTick
  (params (DeltaSeconds :type Float%20%28single-precision%29))
  (if (Variables|Default|GetSeenPlayer?)
    (if (Variables|Default|GetIsAttacking?)
      (Class|NavMovementComponent|StopActiveMovement (Variables|Character|GetCharacterMovement))
      (else
        (CallFunction|ChasePlayer)))))

(fn ConstructionScript)